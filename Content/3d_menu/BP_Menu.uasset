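; BP_Menu is a 3D menu actor that hosts a widget and moves the player's view between linked menu actors.
; On BeginPlay it binds to the widget's TransitionToLinkedMenu event, whose index selects an entry from LinkedMenus.
; A transition disables this actor's collision, enables the target's, and smoothly blends the player camera to the target menu with SetViewTargetWithBlend.
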(event Custom|TransitionTo
  (params (NewMenu :type BP%20Menu%20Object%20Reference))
  (Collision|SetActorEnableCollision false)
  (Collision|SetActorEnableCollision NewMenu true)
  (Game|Player|SetViewTargetwithBlend (Game|GetPlayerController 0) NewMenu 2.0 "VTBlend_EaseInOut" 2.0 false))

(event Custom|ChangeToMenu
  (params (NewParam :type Integer))
  (if (Utilities|Array|IsValidIndex (Variables|Default|GetLinkedMenus) NewParam)
    (CallFunction|Transitionto (Utilities|Array|Get(acopy) (Variables|Default|GetLinkedMenus) NewParam))))

(event EventBeginPlay
  (bind _asmenu_base_widget (Utilities|Casting|CastToMenuBaseWidget (UserInterface|GetUserWidgetObject (Variables|Default|GetWidget))))
  (EventDispatchers|BindEventtoTransitiontoLinkedMenu _asmenu_base_widget (delegate Custom|ChangeToMenu)))

(event Collision|EventActorBeginOverlap
  (params (OtherActor :type Actor%20Object%20Reference)))

(event EventTick
  (params (DeltaSeconds :type Float%20%28single-precision%29)))

(fn ConstructionScript)