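; BP_RootsEnemy is an AI-controlled melee enemy with a health bar widget, facing left or right along X according to its velocity.
; AI Perception writes the sensed Player and line-of-sight flag to the Blackboard, using a timer to delay clearing the flag.
; MeleeAttack spawns a slash effect and damages BP_RootsCharacter actors overlapping the HitBox.
; Incoming damage updates the bar; at zero health it stops movement, plays death FX and destroys itself.
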(event OnTargetPerceptionUpdated(AIPerception)
  (params (Actor :type Actor%20Object%20Reference) (Stimulus :type AI%20Stimulus%20Structure))
  (bind _returnvalue (AI|GetBlackboard 0))
  (if (and (Actor|ActorHasTag Actor "Player") (.bSuccessfullySensed (Utilities|Struct|BreakAIStimulus Stimulus)))
    (Utilities|Time|ClearandInvalidateTimerbyHandle (Variables|Default|GetEnemyTimer))
    (AI|Components|Blackboard|SetValueasBool _returnvalue (Variables|Default|GetHasLineOfSight) true)
    (AI|Components|Blackboard|SetValueasObject _returnvalue (Variables|Default|GetEnemyObj) Actor)
    (else
      (bind _returnvalue_2 (Utilities|Time|SetTimerbyEvent (delegate Custom|StartEnemyTimer) (Variables|Default|GetLineOfSightTimer)))
      (Variables|Default|SetEnemyTimer _returnvalue_2))))

(event Custom|UpdateControllRotation
  (Utilities|IsValid (Pawn|GetController)
    (:Is%20Valid
      (Math|Float|CompareFloat (.X (Math|Vector|BreakVector (Variables|/Script/Engine.MovementComponent|GetVelocity (Variables|Character|GetCharacterMovement)))) 0.0
        (:>
          (Pawn|SetControlRotation (Pawn|GetController) (Math|Rotator|MakeRotator 0.0 0.0 0.0)))
        (:<
          (Pawn|SetControlRotation (Pawn|GetController) (Math|Rotator|MakeRotator 0.0 0.0 1.8e+02)))))))

(event Custom|PlaySpark
  (Niagara|SpawnSystematLocation "/Game/A_Surface_Footstep/Niagara_FX/ParticleSystems/PSN_Sparks_Surface.PSN_Sparks_Surface" (Transformation|GetWorldLocation (Variables|Default|GetNiagara))))

(event Custom|StartEnemyTimer
  (bind _returnvalue (AI|GetBlackboard 0))
  (AI|Components|Blackboard|SetValueasBool _returnvalue (Variables|Default|GetHasLineOfSight) false)
  (AI|Components|Blackboard|SetValueasObject _returnvalue (Variables|Default|GetEnemyObj) (stale OnTargetPerceptionUpdated(AIPerception) Actor)))

(event Custom|MeleeAttack
  (bind _attackeffect (Variables|Default|GetAttackEffect))
  (bind _returnvalue (Transformation|GetWorldTransform _attackeffect))
  (Niagara|SpawnSystematLocation "/Game/Hack_And_Slash_FX/VFX_Niagara/Impacts/NS_Lightning_Slash_Impact.NS_Lightning_Slash_Impact" (.location _returnvalue) (.rotation _returnvalue) (.scale _returnvalue))
  (CallFunction|CheckHit))

(event Custom|CheckHit
  (for _array_element (Collision|GetOverlappingActors (Variables|Default|GetHitBox) "/Game/RootsCharacters/BP_RootsCharacter.BP_RootsCharacter_C" :!class /Script/Engine.PrimitiveComponent)
    (if (!= _array_element self)
      (Game|Damage|ApplyDamage _array_element (Variables|Default|GetBaseDamage) 0 0))))

(event EventBeginPlay
  (bind _asenemy_health_bar (Utilities|Casting|CastToEnemyHealthBar (UserInterface|GetUserWidgetObject (Variables|Default|GetEnemyHealthBar))))
  (Variables|Default|SetHealthWidgetRef _asenemy_health_bar)
  (Variables|/Game/RootsWBP/EnemyHealthBar.EnemyHealthBar_C|SetHealth (Variables|Default|GetHealthWidgetRef) (Variables|Default|GetHealth)))

(event Collision|EventActorBeginOverlap
  (params (OtherActor :type Actor%20Object%20Reference)))

(event Game|Damage|EventAnyDamage
  (params (Damage :type Float%20%28single-precision%29) (DamageType :type Damage%20Type%20Object%20Reference) (InstigatedBy :type Controller%20Object%20Reference) (DamageCauser :type Actor%20Object%20Reference))
  (bind _output_get (Variables|Default|SetHealth (- (Variables|Default|GetHealth) Damage)))
  (Variables|/Game/RootsWBP/EnemyHealthBar.EnemyHealthBar_C|SetHealth (Variables|Default|GetHealthWidgetRef) (Math|Float|Clamp(Float) _output_get 0.0 1e+02))
  (if (<= (Math|Float|Clamp(Float) _output_get 0.0 1e+02) 0.0)
    (Pawn|Components|CharacterMovement|DisableMovement (Variables|Character|GetCharacterMovement))
    (Utilities|FlowControl|Delay 0.3)
    (Niagara|SpawnSystematLocation "/Game/Hack_And_Slash_FX/VFX_Niagara/Impacts/NS_Sakura_Slash_Impact.NS_Sakura_Slash_Impact" (Transformation|GetWorldLocation (Variables|Default|GetDEATHFx)))
    (Development|PrintString "DEATH")
    (Utilities|FlowControl|Delay 0.5)
    (Actor|DestroyActor)))

(event EventTick
  (params (DeltaSeconds :type Float%20%28single-precision%29))
  (CallFunction|UpdateControllRotation))

(fn ConstructionScript)