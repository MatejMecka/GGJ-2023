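; Enemy pawn that chases the BP_RootsCharacter player and fires bullets at them.
; Pawn sensing stores the sighted character as Target and issues an AI move toward it, stopping short at a set radius.
; Without waiting for the move to finish, it turns toward Target and calls Shoot after a delay.
; Shoot aims the spawn point at Target's capsule and spawns a bullet; ShootBullet is an empty stub.
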(event OnSeePawn(PawnSensing)
  (params (Pawn :type Pawn%20Object%20Reference))
  (bind _asbp_roots_character (Utilities|Casting|CastToBP_RootsCharacter Pawn))
  (Variables|Default|SetTarget _asbp_roots_character)
  (AI|AIMoveTo self "0, 0, 0" Pawn 5e+02 false
    (:then
      (Transformation|SetActorRotation (Math|Rotator|FindLookatRotation (Transformation|GetActorLocation self) (Transformation|GetActorLocation (Variables|Default|GetTarget))))
      (Utilities|FlowControl|Delay 1.0)
      (CallFunction|Shoot))))

(event Custom|Shoot
  (bind _target (Variables|Default|GetTarget))
  (Utilities|IsValid _target
    (:Is%20Valid
      (Transformation|SetWorldRotation (Variables|Default|GetProjectile%20Spawn) (Math|Rotator|FindLookatRotation (Transformation|GetWorldLocation (Variables|Default|GetProjectile%20Spawn)) (Transformation|GetWorldLocation (Variables|/Script/Engine.Character|GetCapsuleComponent _target))) false false)
      (Game|SpawnActorfromClass "/Game/ShootingTurret/BulletBluePrint.BulletBluePrint_C" (Transformation|GetWorldTransform (Variables|Default|GetProjectile%20Spawn)) "AlwaysSpawn" 0 0))))

(event EventTick
  (params (DeltaSeconds :type Float%20%28single-precision%29)))

(fn ConstructionScript)

(fn ShootBullet)